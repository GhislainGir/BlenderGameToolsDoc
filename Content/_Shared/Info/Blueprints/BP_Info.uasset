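; BP_Info is an actor that displays configurable text on a pair of planes, apparently as an info board.
; Its construction script copies Text to two text renderers and scales both planes by Height and Width.
; It raises the Scene component in proportion to Height and keeps Plane2 a fixed offset above that.
; The script also sets the actor's location to a fixed world point above the origin.
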(fn `UserConstructionScript`
  (bind _height (`self.Height`))
  (bind _returnvalue (* _height 50.0))
  (`TextRenderComponent.K2_SetText` (`self.TextRender`) (`KismetTextLibrary.Conv_StringToText` (`self.Text`)))
  (`TextRenderComponent.K2_SetText` (`self.TextRender1`) (`KismetTextLibrary.Conv_StringToText` (`self.Text`)))
  (`SceneComponent.SetWorldScale3D` (`self.Plane`) (`KismetMathLibrary.MakeVector` _height (`self.Width`) 1.0))
  (`SceneComponent.SetWorldScale3D` (`self.Plane1`) (`KismetMathLibrary.MakeVector` _height (`self.Width`) 1.0))
  (`SceneComponent.K2_SetRelativeLocation` (`self.Scene`) (`KismetMathLibrary.MakeVector` 0.0 0.0 _returnvalue) false false)
  (`SceneComponent.K2_SetRelativeLocation` (`self.Plane2`) (`KismetMathLibrary.MakeVector` 0.0 0.0 (+ _returnvalue 50.0)) false false)
  (`self.K2_SetActorLocation` (0.0 0.0 150.0)))